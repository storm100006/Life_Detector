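; Construction-script builder that lays out a pipe along the PipePath spline in the level.
; It adds a JointElement static mesh at every spline point and stretches a PipeElement spline mesh between neighbouring points using their tangents.
; A pass for extra meshes at distances along the spline has an empty loop range and unset inputs.
; DrawSplineIndicies optionally labels each point's index with offset text components.
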(event EventBeginPlay)

(event Collision|EventActorBeginOverlap
  (params (OtherActor :type Actor%20Object%20Reference)))

(event EventTick
  (params (DeltaSeconds :type Float%20%28single-precision%29)))

(fn ConstructionScript
  (bind (_x _y _z) (Math|Vector|BreakVector "0, 0, 0"))
  (bind _pipepath (Variables|Default|GetPipePath))
  (bind _pipepath_2 (Variables|Default|GetPipePath))
  (bind _pipepath_3 (Variables|Default|GetPipePath))
  (bind _pipepath_4 (Variables|Default|GetPipePath))
  (bind _returnvalue (Spline|GetSplineLength _pipepath_4))
  (bind _returnvalue_2 (* _returnvalue 0.0))
  (bind _returnvalue_3 (Spline|GetLocationatDistanceAlongSpline _pipepath_3 _returnvalue_2 "World"))
  (Utilities|FlowControl|Sequence
    (:then_0
      (LocalVariables|SetLocal_Num_Spline%20_Points (Spline|GetNumberOfSplinePoints (Variables|Default|GetPipePath)))
      (LocalVariables|SetLocal_Spline_World_Transform (Transformation|GetWorldTransform (Variables|Default|GetPipePath))))
    (:then_1
      (for _index (range 0 (LocalVariables|GetLocal_Num_Spline%20_Points))
        (Math|Integer|CompareInt 0 (LocalVariables|GetLocal_Num_Spline%20_Points))))
    (:then_2
      (for _index_2 (range 0 (- (LocalVariables|GetLocal_Num_Spline%20_Points) 1))
        (LocalVariables|SetLocal_Current_Joint_Index _index_2)
        (if true
          (bind _returnvalue_4 (AddComponent|AddStaticMeshComponent false))
          (Components|StaticMesh|SetStaticMesh _returnvalue_4 (Variables|Default|GetJoint%20Element))
          (Transformation|SetWorldTransform _returnvalue_4 (Math|Transform|ComposeTransforms (Math|Transform|MakeTransform "0, 0, 0" (Math|Rotator|MakeRotator 0.0 0.0 0.0)) (Spline|GetTransformatSplinePoint (Variables|Default|GetPipePath) (LocalVariables|GetLocal_Current_Joint_Index) "World" false)) false false))))
    (:then_3
      (for _index_3 (range 0 (- (LocalVariables|GetLocal_Num_Spline%20_Points) 2))
        (LocalVariables|SetLocal_Current_Spine_Index _index_3)
        (bind _returnvalue_5 (AddComponent|AddSplineMeshComponent false))
        (bind _output_get (LocalVariables|SetLocal_Current_Spline_Mesh _returnvalue_5))
        (Components|StaticMesh|SetStaticMesh _output_get (Variables|Default|GetPipe%20Element))
        (SplineMesh|SetStartandEnd _output_get (.Location (Spline|GetLocationandTangentatSplinePoint _pipepath (LocalVariables|GetLocal_Current_Spine_Index) "Local")) (.Tangent (Spline|GetLocationandTangentatSplinePoint _pipepath (LocalVariables|GetLocal_Current_Spine_Index) "Local")) (.Location (Spline|GetLocationandTangentatSplinePoint _pipepath (+ (LocalVariables|GetLocal_Current_Spine_Index) 1) "Local")) (.Tangent (Spline|GetLocationandTangentatSplinePoint _pipepath (+ (LocalVariables|GetLocal_Current_Spine_Index) 1) "Local")) true :!class /Script/Engine.SplineMeshComponent)))
    (:then_4
      (for _index_4 (range 0 (- 0 1))
        (LocalVariables|SetLocal_Current_AddActorIndex _index_4)
        (Utilities|IsValid 0
          (:Is%20Valid
            (bind _returnvalue_6 (AddComponent|AddStaticMeshComponent false))
            (Components|StaticMesh|SetStaticMesh _returnvalue_6 0)
            (Transformation|SetWorldTransform _returnvalue_6 (Math|Transform|ComposeTransforms (Math|Transform|MakeTransform "0, 0, 0" (Math|Rotator|MakeRotator _x _y _z)) (Math|Transform|MakeTransform _returnvalue_3 (Math|Conversions|RotationFromXVector (- (Spline|GetLocationatDistanceAlongSpline _pipepath_3 (+ _returnvalue_2 0.01) "World") _returnvalue_3)))) false false)))))
    (:then_5
      (if (Variables|Default|GetDraw%20Spline%20Indicies)
        (for _index_5 (range 0 (- (Spline|GetNumberOfSplinePoints _pipepath_2) 1))
          (bind _returnvalue_7 (AddComponent|AddTextRenderComponent false (Math|Transform|MakeTransform (+ (.Location (Spline|GetLocationandTangentatSplinePoint _pipepath_2 _index_5 "Local")) (* (Class|SplineComponent|GetUpVectoratSplinePoint _pipepath_2 _index_5 "Local") (Variables|Default|GetIndicies%20Offset))) (Math|Conversions|RotationFromXVector (* (.Tangent (Spline|GetLocationandTangentatSplinePoint _pipepath_2 _index_5 "Local")) -1.0)))))
          (Rendering|Components|TextRender|SetText _returnvalue_7 (Utilities|Text|ToText(Integer) _index_5)))))))