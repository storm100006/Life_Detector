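; Lantern actor for the canyon landscape that gives off a flickering point light.
; Each Tick calls Play on a timeline, whose LightFlicker track multiplies the Intensity variable to set the light's brightness.
; The construction script applies the base Intensity, while the node for setting the light's color from Lightcolor is left unconnected and never runs.
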(event EventBeginPlay)

(event Collision|EventActorBeginOverlap
  (params (OtherActor :type Actor%20Object%20Reference)))

(event EventTick
  (params (DeltaSeconds :type Float%20%28single-precision%29))
  (bind _lightflicker (Timeline|Timeline_0 Play)
    (:Update
      (Rendering|Components|Light|SetIntensity (Variables|Default|GetPointLight) (* _lightflicker (Variables|Lightsettings|GetIntensity))))))

(fn ConstructionScript
  (Rendering|Components|Light|SetIntensity (Variables|Default|GetPointLight) (Variables|Lightsettings|GetIntensity)))