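; Construction-script actor that scatters static meshes along its Path spline, driven by the InstanceData array.
; Each entry spaces its count evenly over the spline length, with random jitter, a distance offset and optional removal of the last item.
; Each copy is a separate StaticMeshComponent, not a true instance, aligned to spline right/up vectors with rotation, position offset and scale.
; EnableCollisions toggles collision on the spline component only.
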(event OnComponentHit(Path)
  (params (HitComponent :type Primitive%20Component%20Object%20Reference) (OtherActor :type Actor%20Object%20Reference) (OtherComp :type Primitive%20Component%20Object%20Reference) (NormalImpulse :type Vector :default "0, 0, 0") (Hit :type Hit%20Result%20Structure%20%28by%20ref%29)))

(event EventBeginPlay)

(event Collision|EventActorBeginOverlap
  (params (OtherActor :type Actor%20Object%20Reference)))

(event EventTick
  (params (DeltaSeconds :type Float%20%28single-precision%29)))

(fn ConstructionScript
  (bind _path (Variables|Default|GetPath))
  (bind _path_2 (Variables|Default|GetPath))
  (Utilities|FlowControl|Sequence
    (:then_0
      (LocalVariables|SetLocal_SplineLength (Spline|GetSplineLength _path))
      (LocalVariables|SetLocal_SplineTransform (Transformation|GetWorldTransform _path)))
    (:then_1
      (for _array_element (Variables|Default|GetInstanceData)
        (LocalVariables|SetLocal_Mesh (.staticmesh (Utilities|Array|Get(acopy) (Utilities|Array|MakeArray _array_element))))
        (LocalVariables|SetLocal_Count (.count (Utilities|Array|Get(acopy) (Utilities|Array|MakeArray _array_element))))
        (LocalVariables|SetLocal_Spread (/ (LocalVariables|GetLocal_SplineLength) (Math|Conversions|ToFloat(Integer) (- (.count (Utilities|Array|Get(acopy) (Utilities|Array|MakeArray _array_element))) 1))))
        (LocalVariables|SetLocal_RandomLocation (.randomlocation (Utilities|Array|Get(acopy) (Utilities|Array|MakeArray _array_element))))
        (LocalVariables|SetLocal_PositionOffset (.positionoffset (Utilities|Array|Get(acopy) (Utilities|Array|MakeArray _array_element))))
        (LocalVariables|SetLocal_CurrentRotation (.rotation (Utilities|Array|Get(acopy) (Utilities|Array|MakeArray _array_element))))
        (LocalVariables|SetLocal_CurrentScale (.scale (Utilities|Array|Get(acopy) (Utilities|Array|MakeArray _array_element))))
        (LocalVariables|SetLocal_LocationOffset (.locationoffset (Utilities|Array|Get(acopy) (Utilities|Array|MakeArray _array_element))))
        (LocalVariables|SetLocal_RemoveLast (.removelast (Utilities|Array|Get(acopy) (Utilities|Array|MakeArray _array_element))))
        (LocalVariables|SetLocal_LastIndex (- (LocalVariables|GetLocal_Count) (select (LocalVariables|GetLocal_RemoveLast) 2 1)))
        (for _index (range 0 (LocalVariables|GetLocal_LastIndex))
          (LocalVariables|SetLocal_DistanceAlongSpline (+ (* _index (LocalVariables|GetLocal_Spread)) (Math|Random|RandomFloatinRange (* (LocalVariables|GetLocal_RandomLocation) -1.0) (LocalVariables|GetLocal_RandomLocation)) (LocalVariables|GetLocal_LocationOffset)))
          (Utilities|FlowControl|Sequence
            (:then_0
              (bind _returnvalue (AddComponent|AddStaticMeshComponent false))
              (Components|StaticMesh|SetStaticMesh _returnvalue (LocalVariables|GetLocal_Mesh))
              (LocalVariables|SetLocal_StaticMeshComponent _returnvalue))
            (:then_1
              (LocalVariables|SetLocal_FinalPosition (Spline|GetLocationatDistanceAlongSpline (Variables|Default|GetPath) (LocalVariables|GetLocal_DistanceAlongSpline) "Local")))
            (:then_2
              (LocalVariables|SetLocal_FinalRotation (Class|KismetMathLibrary|MakeRotfromYZ (Class|SplineComponent|GetRightVectoratDistanceAlongSpline _path_2 (LocalVariables|GetLocal_DistanceAlongSpline) "Local") (Class|SplineComponent|GetUpVectoratDistanceAlongSpline _path_2 (LocalVariables|GetLocal_DistanceAlongSpline) "Local"))))
            (:then_3
              (Transformation|SetWorldTransform (LocalVariables|GetLocal_StaticMeshComponent) (Math|Transform|ComposeTransforms (Math|Transform|ComposeTransforms (Math|Transform|MakeTransform "0, 0, 0" (Math|Rotator|MakeRotator (.X (Math|Vector|BreakVector (LocalVariables|GetLocal_CurrentRotation))) (.Y (Math|Vector|BreakVector (LocalVariables|GetLocal_CurrentRotation))) (.Z (Math|Vector|BreakVector (LocalVariables|GetLocal_CurrentRotation))))) (Math|Transform|ComposeTransforms (Math|Transform|MakeTransform (LocalVariables|GetLocal_PositionOffset)) (Math|Transform|MakeTransform (LocalVariables|GetLocal_FinalPosition) (LocalVariables|GetLocal_FinalRotation) (LocalVariables|GetLocal_CurrentScale)))) (LocalVariables|GetLocal_SplineTransform)) false false))))))
    (:then_2
      (Collision|SetCollisionEnabled (Variables|Default|GetPath) (select (Variables|Default|GetEnable%20Collisions) "QueryAndPhysics" "NoCollision")))))